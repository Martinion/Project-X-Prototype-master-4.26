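; KillFloor is an actor that damages the player character on overlap and stages a fall camera.
; On overlap it applies damage, caches the character and its spring arm, detaches the arm in world space and plays a scream at the mesh.
; Tick then turns the detached arm toward the character's mesh, so the camera stays behind and watches the body.
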(event `self.ReceiveTick`
  (params (DeltaSeconds :type "Float (single-precision)"))
  (bind _playercharacterref (`self.PlayerCharacterRef`))
  (bind _springarmref (`self.SpringArmRef`))
  (if (and (`KismetSystemLibrary.IsValid` _springarmref) (`KismetSystemLibrary.IsValid` _playercharacterref))
    (`SceneComponent.K2_SetRelativeRotation` _springarmref (`KismetMathLibrary.FindLookAtRotation` (`SceneComponent.K2_GetComponentLocation` _springarmref) (`SceneComponent.K2_GetComponentLocation` (`Character.Mesh` _playercharacterref))) false false)))

(event `self.ReceiveActorBeginOverlap`
  (params (OtherActor :type "Actor Object Reference"))
  (bind _asproto_player_character (cast `/Game/Characters/PlayerCharacter/Proto_Player_Character` OtherActor))
  (`/Game/Characters/PlayerCharacter/Proto_Player_Character.TakeDamage` _asproto_player_character 1.0)
  (bind _output_get (set `self.PlayerCharacterRef` _asproto_player_character))
  (bind _output_get_2 (set `self.SpringArmRef` (`/Game/Characters/PlayerCharacter/Proto_Player_Character.SpringArm` _asproto_player_character)))
  (`SceneComponent.K2_DetachFromComponent` _output_get_2 "KeepWorld" "KeepRelative" "KeepRelative" true)
  (`GameplayStatics.PlaySoundAtLocation` "/Game/Sound/243381__johnsonbrandediting__human-male-scream-3.243381__johnsonbrandediting__human-male-scream-3" (`SceneComponent.K2_GetComponentLocation` (`Character.Mesh` _output_get)) (struct) 1.0 1.0 0.0 null null null))

(fn `UserConstructionScript`)